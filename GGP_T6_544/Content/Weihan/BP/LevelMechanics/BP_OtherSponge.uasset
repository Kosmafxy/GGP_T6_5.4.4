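; BP_OtherSponge is a level-mechanic sponge that swells when a projectile hits it.
; Its Box overlap accepts only BP_Projectile_Base actors and calls AbsorbLiquid, which plays a timeline from the start.
; Each update lerps the Cube's current world scale toward a fixed large size and teleports the actor by LocationOffset, so movement accumulates per update.
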(event OnComponentBeginOverlap(Box)
  (params (OverlappedComponent :type Primitive%20Component%20Object%20Reference) (OtherActor :type Actor%20Object%20Reference) (OtherComp :type Primitive%20Component%20Object%20Reference) (OtherBodyIndex :type Integer) (bFromSweep :type Boolean) (SweepResult :type Hit%20Result%20Structure%20%28by%20ref%29))
  (Utilities|Casting|CastToBP_Projectile_Base OtherActor)
  (CallFunction|AbsorbLiquid))

(event Custom|AbsorbLiquid
  (bind _cube (Variables|Default|GetCube))
  (bind _新建轨道_0 (Timeline|时间轴 PlayFromStart)
    (:Update
      (Transformation|SetWorldScale3D _cube (Math|Vector|Lerp(Vector) (Transformation|GetWorldScale _cube) "60.000000,60.000000,60.000000" _新建轨道_0))
      (Transformation|AddActorWorldOffset (Variables|Default|GetLocationOffset) false true))))

(event EventBeginPlay)

(event Collision|EventActorBeginOverlap
  (params (OtherActor :type Actor%20Object%20Reference)))

(event EventTick
  (params (DeltaSeconds :type Float%20%28single-precision%29)))

(fn ConstructionScript)