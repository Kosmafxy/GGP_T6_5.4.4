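; Switch actor that, when a water projectile overlaps its box, flattens itself on Y and slides linked plane actors to new positions.
; Two timelines drive Plane and Plane2 toward hard-coded world X targets, lerping from each plane's current location every update.
; The Plane3 branch ends in an empty DoOnce, and the Y-axis movement logic for Plane3, Plane4 and Plane5 is disconnected.
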(event OnComponentBeginOverlap(Box)
  (params (OverlappedComponent :type Primitive%20Component%20Object%20Reference) (OtherActor :type Actor%20Object%20Reference) (OtherComp :type Primitive%20Component%20Object%20Reference) (OtherBodyIndex :type Integer) (bFromSweep :type Boolean) (SweepResult :type Hit%20Result%20Structure%20%28by%20ref%29))
  (bind _returnvalue (Transformation|GetActorScale3D))
  (bind _plane (Variables|Default|Getplane))
  (bind _plane2 (Variables|Default|Getplane2))
  (bind _returnvalue_2 (Transformation|GetActorLocation _plane))
  (bind _returnvalue_3 (Transformation|GetActorLocation _plane2))
  (Utilities|Casting|CastToBP_Projectile_Water OtherActor)
  (Transformation|SetActorScale3D (Math|Vector|MakeVector (.x _returnvalue) (* (.y _returnvalue) 0.4) (.z _returnvalue)))
  (Utilities|FlowControl|Sequence
    (:then_0
      (Utilities|IsValid _plane
        (:Is%20Valid
          ;[1 1 1] different plane
          (bind _move_value (Timeline|时间轴 Play)
            (:Update
              (Transformation|SetActorLocationAndRotation _plane (Math|Vector|MakeVector (Math|Float|Lerp (.x _returnvalue_2) 10946.082674 _move_value) (.y _returnvalue_2) (.z _returnvalue_2)) (Transformation|GetActorRotation _plane)))))))
    (:then_1
      (Utilities|IsValid _plane2
        (:Is%20Valid
          (bind _move_value_2 (Timeline|时间轴_0 Play)
            (:Update
              (Transformation|SetActorLocationAndRotation _plane2 (Math|Vector|MakeVector (Math|Float|Lerp (.x _returnvalue_3) -7471.159635 _move_value_2) (.y _returnvalue_3) (.z _returnvalue_3)) (Transformation|GetActorRotation _plane2)))))))
    (:then_2
      (Utilities|IsValid (Variables|Default|Getplane3)
        (:Is%20Valid
          (Utilities|FlowControl|DoOnce false
            (:Completed
              (if true
                _))))))))

(event EventBeginPlay)

(event Collision|EventActorBeginOverlap
  (params (OtherActor :type Actor%20Object%20Reference)))

(event EventTick
  (params (DeltaSeconds :type Float%20%28single-precision%29)))

(fn ConstructionScript)