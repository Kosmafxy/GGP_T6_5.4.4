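; Water-triggered bridge switch that slides one of three referenced plane actors at a time along world Y.
; A BP_Projectile_Water overlapping one of three boxes shrinks this actor's Y scale and plays a timeline lerping the matching plane to a hardcoded Y.
; Each timeline update also returns the other two planes to BeginPlay's hardcoded start locations in two delayed jumps.
; Timer-based SmoothReset events are never called here, and many older return attempts remain disconnected.
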(event OnComponentBeginOverlap(Box)
  (params (OverlappedComponent :type Primitive%20Component%20Object%20Reference) (OtherActor :type Actor%20Object%20Reference) (OtherComp :type Primitive%20Component%20Object%20Reference) (OtherBodyIndex :type Integer) (bFromSweep :type Boolean) (SweepResult :type Hit%20Result%20Structure%20%28by%20ref%29))
  (bind _returnvalue (Transformation|GetActorScale3D))
  (bind _plane2 (Variables|Default|Getplane2))
  (bind _plane4_startlocation (Variables|Default|GetPlane4_StartLocation))
  (bind _plane3_startlocation (Variables|Default|GetPlane3_StartLocation))
  (bind _returnvalue_2 (Transformation|GetActorLocation _plane2))
  ;[1 1 1] valid
  (Utilities|Casting|CastToBP_Projectile_Water OtherActor)
  (Transformation|SetActorScale3D (Math|Vector|MakeVector (.x _returnvalue) (* (.y _returnvalue) 0.8) (.z _returnvalue)))
  (Utilities|IsValid _plane2
    (:Is%20Valid
      (bind _move_value (Timeline|时间轴_2 PlayFromStart)
        (:Update
          (Transformation|SetActorLocationAndRotation _plane2 (Math|Vector|MakeVector (.x _returnvalue_2) (Math|Float|Lerp (.y _returnvalue_2) -34313.837332 _move_value) (.z _returnvalue_2)) (Transformation|GetActorRotation _plane2))
          (Utilities|FlowControl|Sequence
            (:then_0
              (if (not (== (.y (Transformation|GetActorLocation (Variables|Default|Getplane))) (.y _plane3_startlocation)))
                (Utilities|FlowControl|Delay 1.0)
                (Transformation|SetActorLocation (Variables|Default|Getplane) (Math|Vector|MakeVector (.x _plane3_startlocation) (- (.y _plane3_startlocation) (Variables|Default|GetNewVar)) (.z _plane3_startlocation)) false false)
                (Utilities|FlowControl|Delay 1.0)
                (Transformation|SetActorLocation (Variables|Default|Getplane) (Variables|Default|GetPlane3_StartLocation) false false)))
            (:then_1
              (if (not (== (.y (Transformation|GetActorLocation (Variables|Default|Getplane1))) (.y _plane4_startlocation)))
                (Utilities|FlowControl|Delay 1.0)
                (Transformation|SetActorLocation (Variables|Default|Getplane1) (Math|Vector|MakeVector (.x _plane4_startlocation) (+ (.y _plane4_startlocation) 2e+02) (.z _plane4_startlocation)) false false)
                (Utilities|FlowControl|Delay 1.0)
                (Transformation|SetActorLocation (Variables|Default|Getplane1) (Variables|Default|GetPlane4_StartLocation) false false)))))))))

(event OnComponentBeginOverlap(Box1)
  (params (OverlappedComponent :type Primitive%20Component%20Object%20Reference) (OtherActor :type Actor%20Object%20Reference) (OtherComp :type Primitive%20Component%20Object%20Reference) (OtherBodyIndex :type Integer) (bFromSweep :type Boolean) (SweepResult :type Hit%20Result%20Structure%20%28by%20ref%29))
  (bind _returnvalue (Transformation|GetActorScale3D))
  (bind _plane1 (Variables|Default|Getplane1))
  (bind _plane5_startlocation (Variables|Default|GetPlane5_StartLocation))
  (bind _plane3_startlocation (Variables|Default|GetPlane3_StartLocation))
  (bind _returnvalue_2 (Transformation|GetActorLocation _plane1))
  ;[1 1 1] valid
  (Utilities|Casting|CastToBP_Projectile_Water OtherActor)
  (Transformation|SetActorScale3D (Math|Vector|MakeVector (.x _returnvalue) (* (.y _returnvalue) 0.8) (.z _returnvalue)))
  (Utilities|IsValid _plane1
    (:Is%20Valid
      (bind _move_value (Timeline|时间轴 PlayFromStart)
        (:Update
          (Transformation|SetActorLocationAndRotation _plane1 (Math|Vector|MakeVector (.x _returnvalue_2) (Math|Float|Lerp (.y _returnvalue_2) -34992.92262 _move_value) (.z _returnvalue_2)) (Transformation|GetActorRotation _plane1))
          (Utilities|FlowControl|Sequence
            (:then_0
              (if (not (== (.y (Transformation|GetActorLocation (Variables|Default|Getplane))) (.y _plane3_startlocation)))
                (Utilities|FlowControl|Delay 1.0)
                (Transformation|SetActorLocation (Variables|Default|Getplane) (Math|Vector|MakeVector (.x _plane3_startlocation) (- (.y _plane3_startlocation) (Variables|Default|GetNewVar)) (.z _plane3_startlocation)) false false)
                (Utilities|FlowControl|Delay 1.0)
                (Transformation|SetActorLocation (Variables|Default|Getplane) (Variables|Default|GetPlane3_StartLocation) false false)))
            (:then_1
              (if (not (== (.y (Transformation|GetActorLocation (Variables|Default|Getplane2))) (.y _plane5_startlocation)))
                (Utilities|FlowControl|Delay 1.0)
                (Transformation|SetActorLocation (Variables|Default|Getplane2) (Math|Vector|MakeVector (.x _plane5_startlocation) (- (.y _plane5_startlocation) (Variables|Default|GetNewVar)) (.z _plane5_startlocation)) false false)
                (Utilities|FlowControl|Delay 1.0)
                (Transformation|SetActorLocation (Variables|Default|Getplane2) (Variables|Default|GetPlane5_StartLocation) false false)))))))))

(event OnComponentBeginOverlap(Box2)
  (params (OverlappedComponent :type Primitive%20Component%20Object%20Reference) (OtherActor :type Actor%20Object%20Reference) (OtherComp :type Primitive%20Component%20Object%20Reference) (OtherBodyIndex :type Integer) (bFromSweep :type Boolean) (SweepResult :type Hit%20Result%20Structure%20%28by%20ref%29))
  (bind _returnvalue (Transformation|GetActorScale3D))
  (bind _plane5_startlocation (Variables|Default|GetPlane5_StartLocation))
  (bind _plane4_startlocation (Variables|Default|GetPlane4_StartLocation))
  (bind _plane (Variables|Default|Getplane))
  (bind _returnvalue_2 (Transformation|GetActorLocation _plane))
  ;[1 1 1] valid
  (Utilities|Casting|CastToBP_Projectile_Water OtherActor)
  (Transformation|SetActorScale3D (Math|Vector|MakeVector (.x _returnvalue) (* (.y _returnvalue) 0.8) (.z _returnvalue)))
  (Utilities|IsValid _plane
    (:Is%20Valid
      (bind _move_value (Timeline|时间轴_3 PlayFromStart)
        (:Update
          (Transformation|SetActorLocationAndRotation _plane (Math|Vector|MakeVector (.x _returnvalue_2) (Math|Float|Lerp (.y _returnvalue_2) -34313.837332 _move_value) (.z _returnvalue_2)) (Transformation|GetActorRotation _plane))
          (Utilities|FlowControl|Sequence
            (:then_0
              (if (not (== (.y (Transformation|GetActorLocation (Variables|Default|Getplane1))) (.y _plane4_startlocation)))
                (Utilities|FlowControl|Delay 1.0)
                (Transformation|SetActorLocation (Variables|Default|Getplane1) (Math|Vector|MakeVector (.x _plane4_startlocation) (+ (.y _plane4_startlocation) 2e+02) (.z _plane4_startlocation)) false false)
                (Utilities|FlowControl|Delay 1.0)
                (Transformation|SetActorLocation (Variables|Default|Getplane1) (Variables|Default|GetPlane4_StartLocation) false false)))
            (:then_1
              (if (not (== (.y (Transformation|GetActorLocation (Variables|Default|Getplane2))) (.y _plane5_startlocation)))
                (Utilities|FlowControl|Delay 1.0)
                (Transformation|SetActorLocation (Variables|Default|Getplane2) (Math|Vector|MakeVector (.x _plane5_startlocation) (- (.y _plane5_startlocation) (Variables|Default|GetNewVar)) (.z _plane5_startlocation)) false false)
                (Utilities|FlowControl|Delay 1.0)
                (Transformation|SetActorLocation (Variables|Default|Getplane2) (Variables|Default|GetPlane5_StartLocation) false false)))))))))

(event Custom|SmoothReset1
  ;[1 1 1] for try
  ;;[1 1 1] 注释
  ;;;[1 1 1] smooth move 1
  (bind _returnvalue (Utilities|Time|SetTimerbyEvent (delegate Custom|_MoveStep1) 0.1 true)))

(event Custom|_MoveStep1
  (bind _plane (Variables|Default|Getplane))
  (bind _plane3_startlocation (Variables|Default|GetPlane3_StartLocation))
  (bind _returnvalue (Transformation|GetActorLocation _plane))
  (bind _returnvalue_2 (Math|Vector|Lerp(Vector) _returnvalue _plane3_startlocation 0.01))
  ;[1 1 1] for try
  ;;[1 1 1] 注释
  ;;;[1 1 1] smooth move 1
  (Transformation|SetActorLocation _returnvalue_2 false false)
  (if (< (Math|Vector|VectorLength _returnvalue_2) 1.0)
    (Utilities|Time|ClearandInvalidateTimerbyHandle (stale Custom|SmoothReset1 _returnvalue))))

(event Custom|_MoveStep
  (bind _plane (Variables|Default|Getplane))
  (bind _plane3_startlocation (Variables|Default|GetPlane3_StartLocation))
  (bind _returnvalue (Transformation|GetActorLocation _plane))
  (bind _returnvalue_2 (Math|Vector|Lerp(Vector) _returnvalue _plane3_startlocation 0.01))
  ;[1 1 1] for try
  ;;[1 1 1] 注释
  ;;;[1 1 1] smooth move 1
  (Transformation|SetActorLocation _returnvalue_2 false false)
  (if (< (Math|Vector|VectorLength _returnvalue_2) 1.0)
    (Utilities|Time|ClearandInvalidateTimerbyHandle (stale Custom|SmoothReset _returnvalue))))

(event Custom|SmoothReset
  ;[1 1 1] for try
  ;;[1 1 1] 注释
  ;;;[1 1 1] smooth move 1
  (bind _returnvalue (Utilities|Time|SetTimerbyEvent (delegate Custom|_MoveStep) 0.1 true)))

(event EventBeginPlay
  ;[1 1 1] valid
  (Variables|Default|SetPlane3_StartLocation "21806.542938,-33664.884179,3530.672641")
  (Variables|Default|SetPlane4_StartLocation "21399.409638,-35621.476294,3530.672648")
  (Variables|Default|SetPlane5_StartLocation "20962.601601,-33664.884178,3530.672642"))

(event Collision|EventActorBeginOverlap
  (params (OtherActor :type Actor%20Object%20Reference)))

(event EventTick
  (params (DeltaSeconds :type Float%20%28single-precision%29))
  ;[1 1 1] for try
)

(fn ConstructionScript)