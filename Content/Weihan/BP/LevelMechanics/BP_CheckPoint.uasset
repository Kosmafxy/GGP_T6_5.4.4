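; BP_CheckPoint is a one-shot checkpoint that updates the player's respawn location.
; When BP_Cube_Player overlaps its Box, it writes the checkpoint's location to both BP_SpongeGameInstance and the player.
; It prints the location, then destroys itself after a short delay.
; An unconnected chain that would move the PlayerStart never runs.
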(event OnComponentBeginOverlap(Box)
  (params (OverlappedComponent :type Primitive%20Component%20Object%20Reference) (OtherActor :type Actor%20Object%20Reference) (OtherComp :type Primitive%20Component%20Object%20Reference) (OtherBodyIndex :type Integer) (bFromSweep :type Boolean) (SweepResult :type Hit%20Result%20Structure%20%28by%20ref%29))
  (bind _returnvalue (Transformation|GetActorTransform))
  (bind _asbp_cube_player (Utilities|Casting|CastToBP_Cube_Player OtherActor))
  (bind _asbp_sponge_game_instance (Utilities|Casting|CastToBP_SpongeGameInstance (Game|GetGameInstance))
    (:then
      _)
    (:CastFailed
      _))
  (Variables|/Game/Weihan/BP_SpongeGameInstance.BP_SpongeGameInstance_C|SetPlayer_RespawnLocation _asbp_sponge_game_instance (.location _returnvalue))
  (bind _output_get (Variables|/Game/Weihan/BP/Character/BP_Cube_Player.BP_Cube_Player_C|SetRespawnLocation _asbp_cube_player (.location _returnvalue)))
  (Development|PrintString (Utilities|String|ToString(Vector) _output_get))
  (Utilities|FlowControl|Delay 0.2)
  (Actor|DestroyActor))

(event EventBeginPlay)

(event Collision|EventActorBeginOverlap
  (params (OtherActor :type Actor%20Object%20Reference)))

(event EventTick
  (params (DeltaSeconds :type Float%20%28single-precision%29)))

(fn ConstructionScript)