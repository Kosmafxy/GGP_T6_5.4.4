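; BP_Enemy_Elite is an elite enemy that hurts the cube player on contact and can be killed by damage.
; Its capsule overlap applies a small fixed damage to BP_Cube_Player, passing its controller as both instigator and damage causer.
; Incoming damage is truncated to an integer and subtracted from Health, and Death destroys the actor once Health reaches -2 or lower, rather than zero.
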(event OnComponentBeginOverlap(CapsuleComponent)
  (params (OverlappedComponent :type Primitive%20Component%20Object%20Reference) (OtherActor :type Actor%20Object%20Reference) (OtherComp :type Primitive%20Component%20Object%20Reference) (OtherBodyIndex :type Integer) (bFromSweep :type Boolean) (SweepResult :type Hit%20Result%20Structure%20%28by%20ref%29))
  (bind _returnvalue (Pawn|GetController))
  (bind _asbp_cube_player (Utilities|Casting|CastToBP_Cube_Player OtherActor))
  (Game|Damage|ApplyDamage _asbp_cube_player 1.0 _returnvalue _returnvalue))

(event EventBeginPlay)

(event Collision|EventActorBeginOverlap
  (params (OtherActor :type Actor%20Object%20Reference)))

(event EventTick
  (params (DeltaSeconds :type Float%20%28single-precision%29)))

(event Game|Damage|EventAnyDamage
  (params (Damage :type Float%20%28single-precision%29) (DamageType :type Damage%20Type%20Object%20Reference) (InstigatedBy :type Controller%20Object%20Reference) (DamageCauser :type Actor%20Object%20Reference))
  (bind _output_get (Variables|Default|SetHealth (- (Variables|Default|GetHealth) (Math|Float|Truncate Damage))))
  (if (<= _output_get -2)
    (CallFunction|Death)))

(fn ConstructionScript)

(fn Death
  (Actor|DestroyActor))