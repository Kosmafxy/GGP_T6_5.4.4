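; Trigger actor that clears a set of referenced actors, including FOG, four seconds after BP_Cube_Player overlaps its Box.
; Actors are destroyed in four groups chained by short delays.
; A Sequence also runs IsValid checks that jump straight into each group, so groups with valid references are destroyed immediately after the initial wait rather than staggered.
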(event OnComponentBeginOverlap(Box)
  (params (OverlappedComponent :type Primitive%20Component%20Object%20Reference) (OtherActor :type Actor%20Object%20Reference) (OtherComp :type Primitive%20Component%20Object%20Reference) (OtherBodyIndex :type Integer) (bFromSweep :type Boolean) (SweepResult :type Hit%20Result%20Structure%20%28by%20ref%29))
  (Utilities|Casting|CastToBP_Cube_Player OtherActor)
  (Utilities|FlowControl|Delay 4.0)
  (Utilities|FlowControl|Sequence
    (:then_0
      (bind _r1_1 (Variables|Default|GetR1-1)
        (:then
          (Actor|DestroyActor _r1_1 :!label _label))
        (:else
          _))
      (Utilities|FlowControl|Delay 0.2 :!label _label_2)
      (Actor|DestroyActor (stale _r1) :!label _label_3)
      (Utilities|FlowControl|Delay 0.2 :!label _label_4)
      (Actor|DestroyActor (stale _s1) :!label _label_5)
      (Utilities|FlowControl|Delay 0.2 :!label _label_6))
    (:then_1
      (bind _r2_2 (Variables|Default|GetR2-2)
        (:then
          (goto _label))
        (:else
          (goto _label_2))))
    (:then_2
      (bind _r3_3 (Variables|Default|GetR3-3)
        (:then
          (goto _label))
        (:else
          (goto _label_2))))
    (:then_3
      (bind _r1 (Variables|Default|GetR1)
        (:then
          (goto _label_3))
        (:else
          (goto _label_4))))
    (:then_4
      (bind _r2 (Variables|Default|GetR2)
        (:then
          (goto _label_3))
        (:else
          (goto _label_4))))
    (:then_5
      (bind _r3 (Variables|Default|GetR3)
        (:then
          (goto _label_3))
        (:else
          (goto _label_4))))
    (:then_6
      (bind _s1 (Variables|Default|GetS1)
        (:then
          (goto _label_5))
        (:else
          (goto _label_6))))
    (:then_7
      (bind _s2 (Variables|Default|GetS2)
        (:then
          (goto _label_5))
        (:else
          (goto _label_6))))
    (:then_8
      (bind _r4 (Variables|Default|GetR4)
        (:then
          _)
        (:else)))
    (:then_9
      (bind _r5 (Variables|Default|GetR5)
        (:then
          _)
        (:else))))
  (Actor|DestroyActor _r4))

(event EventBeginPlay)

(event Collision|EventActorBeginOverlap
  (params (OtherActor :type Actor%20Object%20Reference)))

(event EventTick
  (params (DeltaSeconds :type Float%20%28single-precision%29)))

(fn ConstructionScript)