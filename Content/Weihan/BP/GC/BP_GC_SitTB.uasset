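; BP_GC_SitTB is a breakable prop built on a Geometry Collection that collapses when a liquid-carrying player cube enters its Box volume.
; Tick polls the Box for overlapping BP_Cube_Player actors and crumbles the collection's active clusters for any with HaveLiquid set.
; The Chaos break event plays a 2D wood-cracking sound, gated by DoOnce so it fires only on the first break.
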(event OnChaosBreakEvent(GeometryCollection)
  (params (BreakEvent :type Chaos%20Break%20Event%20Structure%20%28by%20ref%29))
  (Utilities|FlowControl|DoOnce false
    (:Completed
      (Audio|PlaySound2D "/Game/Hang/SFX/S_CrackingWood.S_CrackingWood" 1.0 1.0 0.0 0 0))))

(event EventBeginPlay)

(event Collision|EventActorBeginOverlap
  (params (OtherActor :type Actor%20Object%20Reference)))

(event EventTick
  (params (DeltaSeconds :type Float%20%28single-precision%29))
  (for _array_element (Collision|GetOverlappingActors (Variables|Default|GetBox) "/Game/Weihan/BP/Character/BP_Cube_Player.BP_Cube_Player_C" :!class /Script/Engine.PrimitiveComponent)
    (bind _asbp_cube_player (Utilities|Casting|CastToBP_Cube_Player _array_element))
    (if (Variables|/Game/Weihan/BP/Character/BP_Cube_Player.BP_Cube_Player_C|GetHaveLiquid? _asbp_cube_player)
      (Class|GeometryCollectionComponent|CrumbleActiveClusters (Variables|Default|GetGeometryCollection)))))

(fn ConstructionScript)