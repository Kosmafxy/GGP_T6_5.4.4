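; BP_leverTest is a test seesaw lever that tilts its Board according to the player character's position.
; Tick compares the player's world Y with the Cone pivot's world X, despite the differing axes.
; Outside a small dead zone, that offset, normalized by half the board's length, sets a clamped roll target reached via RInterpTo.
; An unconnected overlap branch would toggle Board physics from BP_Cube_Player's Z scale.
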(event EventBeginPlay
  (Variables|Default|SetCharacter%20Ref (Game|GetPlayerCharacter 0)))

(event Collision|EventActorBeginOverlap
  (params (OtherActor :type Actor%20Object%20Reference)))

(event EventTick
  (params (DeltaSeconds :type Float%20%28single-precision%29))
  (bind _output_get (Variables|Default|SetPlayerLocationX (.y (Transformation|GetActorLocation (Variables|Default|GetCharacter%20Ref)))))
  (bind _output_get_2 (Variables|Default|SetPivotLocationX (.x (Transformation|GetWorldLocation (Variables|Default|Getcone)))))
  (bind _output_get_3 (Variables|Default|SetDistanceFromCenter (- _output_get _output_get_2)))
  (Utilities|FlowControl|Sequence
    (:then_0
      (if (> _output_get_3 5.0)
        (Variables|Default|SetNewSide 1)
        (bind _output_get_4 (Variables|Default|SetNormalized%20Distance (Math|Float|Clamp(Float) (/ _output_get_3 (/ (* (.y (Variables|/Script/Engine.SceneComponent|GetRelativeScale3D (Variables|Default|Getboard))) 1e+02) 2.0)) -1.0) :!label _label))
        (bind _output_get_5 (Variables|Default|SetTargetTiltAngle (* _output_get_4 (Variables|Default|GetMax%20Tilt%20Angle))))
        (bind _output_get_6 (Variables|Default|SetTarget%20Rotation (Math|Rotator|MakeRotator _output_get_5 0.0 0.0)))
        (Transformation|SetRelativeRotation (Variables|Default|Getboard) (Math|Interpolation|RInterpTo (Variables|/Script/Engine.SceneComponent|GetRelativeRotation (Variables|Default|Getboard)) _output_get_6 (Utilities|Time|GetWorldDeltaSeconds) (Variables|Default|GetInterp%20Speed)) false false)
        (if (!= (Variables|Default|GetNewSide) (Variables|Default|GetLast%20Side))
          (bind _output_get_7 (Variables|Default|SetLast%20Side (Math|Conversions|ToInteger(Boolean) (!= (Variables|Default|GetNewSide) (Variables|Default|GetLast%20Side)))))
          (Variables|Default|SetNewSide _output_get_7)
          (Variables|Default|SetTargetTiltAngle (Math|Conversions|ToFloat(Integer) _output_get_7)))
        (else
          (Variables|Default|SetNewSide 0 :!label _label_2))))
    (:then_1
      (if (< _output_get_3 -5.0)
        (Variables|Default|SetNewSide -1)
        (goto _label)
        (else
          (goto _label_2))))))

(fn ConstructionScript)