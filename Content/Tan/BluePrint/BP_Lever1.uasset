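; BP_Lever1 is a lever whose Board becomes physically simulated when a large enough player cube is on it.
; Each Tick it polls OverlapEvent for overlapping BP_Cube_Player actors and enables Board physics if the cube's Z scale exceeds 1, otherwise disables it.
; A DoOnce plays the S_QQB sound the first time physics is enabled.
; With no overlapping cube the loop does nothing, so Board keeps its last physics state.
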(event EventBeginPlay)

(event Collision|EventActorBeginOverlap
  (params (OtherActor :type Actor%20Object%20Reference)))

(event EventTick
  (params (DeltaSeconds :type Float%20%28single-precision%29))
  (bind _board (Variables|Default|Getboard))
  ;[1 1 1] enable lever
  (for _array_element (Collision|GetOverlappingActors (Variables|Default|Getoverlap%20event) "/Game/Weihan/BP/Character/BP_Cube_Player.BP_Cube_Player_C" :!class /Script/Engine.PrimitiveComponent)
    (if (Utilities|IsValid _array_element)
      (bind _asbp_cube_player (Utilities|Casting|CastToBP_Cube_Player _array_element))
      (if (> (.z (Transformation|GetActorScale3D _asbp_cube_player)) 1.0)
        (Physics|SetSimulatePhysics _board true)
        (Utilities|FlowControl|DoOnce false
          (:Completed
            (Audio|PlaySound2D "/Game/Hang/SFX/S_QQB.S_QQB" 1.0 1.0 0.0 0 0)))
        (else
          (Physics|SetSimulatePhysics _board false)))
      (else
        (Physics|SetSimulatePhysics (Variables|Default|Getboard) false)))))

(fn ConstructionScript)