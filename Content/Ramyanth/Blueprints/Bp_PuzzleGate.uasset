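; Puzzle gate Blueprint that swings its door open once enough puzzle items are collected.
; Each CollectItem call increments a counter and compares it to MaxItemsCollected, using DoOnce so the opening triggers a single time.
; A timeline lerps the door's relative yaw to open it.
; BeginPlay stores the count of Bp_PuzzleItem actors in AllOfItem, which the open check does not use.
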(event Custom|OpenDoor
  (bind _door_rotation (Timeline|Open%20Door%20Anim Play)
    (:Update
      (Transformation|SetRelativeRotation (Variables|Default|GetDoor) (Math|Rotator|MakeRotator 0.0 0.0 (Math|Float|Lerp 0.0 1.2e+02 _door_rotation)) false false))))

(event Custom|Collect%20Item
  (Math|Integer|IncrementInt (Variables|Default|GetCurrentItemsCollected)
    (:%20%20
      (CallFunction|OpenDoorCheck))))

(event Custom|Open%20Door%20Check
  (if (>= (Variables|Default|GetCurrentItemsCollected) (Variables|Default|GetMaxItemsCollected))
    (Utilities|FlowControl|DoOnce false
      (:Completed
        (CallFunction|OpenDoor)))))

(event EventBeginPlay
  (bind _outactors (Actor|GetAllActorsOfClass "/Game/Ramyanth/Blueprints/Bp_PuzzleItem.Bp_PuzzleItem_C"))
  (Variables|Default|SetAll%20Of%20Item (Utilities|Array|Length _outactors)))

(fn ConstructionScript)