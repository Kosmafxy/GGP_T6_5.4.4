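; A painting actor that reacts to projectile hits with a material blend and a cutscene that relocates the player.
; A BP_Projectile_Base overlapping its Box plays a timeline driving the Blend parameter of a Jellfish_Mat dynamic instance on Spawnplace's mesh.
; The timeline's Update also feeds a delay, then hides the player, disables input and plays a level sequence.
; When the sequence finishes, the player moves to a hard-coded location and reappears, without input being re-enabled here.
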(event OnComponentBeginOverlap(Box)
  (params (OverlappedComponent :type Primitive%20Component%20Object%20Reference) (OtherActor :type Actor%20Object%20Reference) (OtherComp :type Primitive%20Component%20Object%20Reference) (OtherBodyIndex :type Integer) (bFromSweep :type Boolean) (SweepResult :type Hit%20Result%20Structure%20%28by%20ref%29))
  (Utilities|Casting|CastToBP_Projectile_Base OtherActor)
  (bind _blend_value (Timeline|时间轴 Play)
    (:Update
      (bind _returnvalue (Rendering|Material|CreateDynamicMaterialInstance (Actor|GetComponentbyClass (Variables|Default|Getspawnplace) "/Script/Engine.StaticMeshComponent") 0 "/Game/Tan/pictures_Li/jellfish_Mat.jellfish_Mat" "Blend" :!class /Script/Engine.PrimitiveComponent))
      (Rendering|Material|SetScalarParameterValue _returnvalue "Blend" _blend_value :!class /Script/Engine.MaterialInstanceDynamic)
      (Utilities|FlowControl|Delay 5.0)
      (Rendering|SetActorHiddenInGame (Game|GetPlayerCharacter 0) true)
      (Input|DisableInput (Game|GetPlayerController 0) 0)
      (bind (_outactor _returnvalue_2) (Sequencer|Player|CreateLevelSequencePlayer "/Game/Tan/NewLevelSequence.NewLevelSequence"))
      (Sequencer|Player|Play (Variables|/Script/LevelSequence.LevelSequenceActor|GetSequencePlayer _outactor) :!class /Script/MovieScene.MovieSceneSequencePlayer)
      (EventDispatchers|BindEventtoOnFinished _returnvalue_2 (delegate Custom|OnCinematicFinished)))))

(event Custom|OnCinematicFinished
  (bind _returnvalue (Game|GetPlayerCharacter 0))
  (Transformation|SetActorLocation _returnvalue "10233.000000,-39341.000000,2940.000000" false false)
  (Rendering|SetActorHiddenInGame _returnvalue false))

(event EventBeginPlay)

(event Collision|EventActorBeginOverlap
  (params (OtherActor :type Actor%20Object%20Reference)))

(event EventTick
  (params (DeltaSeconds :type Float%20%28single-precision%29)))

(fn ConstructionScript)