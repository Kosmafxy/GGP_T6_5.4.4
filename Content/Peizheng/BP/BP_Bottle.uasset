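; BP_Bottle is a bottle actor that reacts to projectiles and to the cube player carrying liquid.
; The first BP_Projectile_Base overlapping its capsule swaps the Water mesh for WaterFull and re-angles the spotlight.
; A player with HaveLiquid entering LightCollision starts a timeline that lerps the player's scale between unit and the bottle's scale, clears HaveLiquid and makes the crosshair transparent.
; A camera pull-back step is left unconnected.
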(event OnComponentBeginOverlap(Capsule)
  (params (OverlappedComponent :type Primitive%20Component%20Object%20Reference) (OtherActor :type Actor%20Object%20Reference) (OtherComp :type Primitive%20Component%20Object%20Reference) (OtherBodyIndex :type Integer) (bFromSweep :type Boolean) (SweepResult :type Hit%20Result%20Structure%20%28by%20ref%29))
  (Utilities|Casting|CastToBP_Projectile_Base OtherActor)
  (Utilities|FlowControl|DoOnce false
    (:Completed
      (Rendering|SetVisibility (Variables|Default|GetWater_full) true false)
      (Rendering|SetVisibility (Variables|Default|GetWater) false false)
      (Transformation|SetRelativeRotation (Variables|Default|GetSpotLight) "-10.000000,0.000000,0.000000" false false))))

(event OnComponentBeginOverlap(LightCollision)
  (params (OverlappedComponent :type Primitive%20Component%20Object%20Reference) (OtherActor :type Actor%20Object%20Reference) (OtherComp :type Primitive%20Component%20Object%20Reference) (OtherBodyIndex :type Integer) (bFromSweep :type Boolean) (SweepResult :type Hit%20Result%20Structure%20%28by%20ref%29))
  (bind _asbp_cube_player (Utilities|Casting|CastToBP_Cube_Player OtherActor))
  (if (Variables|/Game/Weihan/BP/Character/BP_Cube_Player.BP_Cube_Player_C|GetHaveLiquid? _asbp_cube_player)
    (bind _新建轨道_0 (Timeline|时间轴 Play)
      (:Update
        (Transformation|SetActorScale3D _asbp_cube_player (Math|Vector|Lerp(Vector) "1.000000,1.000000,1.000000" (Transformation|GetActorScale3D) _新建轨道_0))
        (Variables|/Game/Weihan/BP/Character/BP_Cube_Player.BP_Cube_Player_C|SetHaveLiquid? _asbp_cube_player false)
        (Appearance|SetColorandOpacity (Variables|/Game/Weihan/BP/Character/BP_Cube_Player.BP_Cube_Player_C|GetCrosshair _asbp_cube_player) "(R=0.000000,G=0.000000,B=0.000000,A=0.000000)" :!class /Script/UMG.UserWidget)))))

(event EventBeginPlay)

(event Collision|EventActorBeginOverlap
  (params (OtherActor :type Actor%20Object%20Reference)))

(event EventTick
  (params (DeltaSeconds :type Float%20%28single-precision%29)))

(fn ConstructionScript)