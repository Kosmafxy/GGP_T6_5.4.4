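; BP_Arrow is a direction trigger that steers BP_Cube_Player when it enters its box.
; A DoOnce-guarded overlap alternates the player's Direction between Left and Right by flipping FirstIsLeft.
; Only the Left branch also snaps the player's rotation to the Left component.
; When the player exits, a half-second delay precedes a "ce Reset" console command and re-arming of the DoOnce.
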(event OnComponentBeginOverlap(Box)
  (params (OverlappedComponent :type Primitive%20Component%20Object%20Reference) (OtherActor :type Actor%20Object%20Reference) (OtherComp :type Primitive%20Component%20Object%20Reference) (OtherBodyIndex :type Integer) (bFromSweep :type Boolean) (SweepResult :type Hit%20Result%20Structure%20%28by%20ref%29))
  (bind _left (Variables|Default|GetLeft))
  (bind _asbp_cube_player (Utilities|Casting|CastToBP_Cube_Player OtherActor))
  (Utilities|FlowControl|DoOnce false
    (:Completed
      (if (Variables|Default|GetFirstIsLeft)
        (Variables|/Game/Weihan/BP/Character/BP_Cube_Player.BP_Cube_Player_C|SetDirection _asbp_cube_player _left)
        (Variables|Default|SetFirstIsLeft false)
        (Transformation|SetActorRotation _asbp_cube_player (Transformation|GetWorldRotation _left))
        (else
          (Variables|/Game/Weihan/BP/Character/BP_Cube_Player.BP_Cube_Player_C|SetDirection _asbp_cube_player (Variables|Default|GetRight))
          (Variables|Default|SetFirstIsLeft true))))))

(event OnComponentEndOverlap(Box)
  (params (OverlappedComponent :type Primitive%20Component%20Object%20Reference) (OtherActor :type Actor%20Object%20Reference) (OtherComp :type Primitive%20Component%20Object%20Reference) (OtherBodyIndex :type Integer))
  (bind _left (Variables|Default|GetLeft))
  (Utilities|Casting|CastToBP_Cube_Player OtherActor)
  (Utilities|FlowControl|Delay 0.5)
  (Development|ExecuteConsoleCommand "ce Reset" 0)
  (Utilities|FlowControl|DoOnce false) ; enters at Reset
)

(event EventBeginPlay)

(event Collision|EventActorBeginOverlap
  (params (OtherActor :type Actor%20Object%20Reference)))

(event EventTick
  (params (DeltaSeconds :type Float%20%28single-precision%29)))

(fn ConstructionScript)