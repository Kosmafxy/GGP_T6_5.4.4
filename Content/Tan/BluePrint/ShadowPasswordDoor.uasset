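; Shadow password door puzzle trigger: when a water projectile or the cube player overlaps its Box, it runs a scripted door-opening sequence.
; Chained timelines and delays raise a steel frame, drive a Blend parameter on a dynamic material, then slide the door along X and destroy it.
; Movement lerps from each actor's current position toward hard-coded world coordinates, and delays and material creation sit inside timeline updates.
; A Fade timeline is left unconnected.
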(event OnComponentBeginOverlap(Box)
  (params (OverlappedComponent :type Primitive%20Component%20Object%20Reference) (OtherActor :type Actor%20Object%20Reference) (OtherComp :type Primitive%20Component%20Object%20Reference) (OtherBodyIndex :type Integer) (bFromSweep :type Boolean) (SweepResult :type Hit%20Result%20Structure%20%28by%20ref%29))
  (bind _steel_frame_movement (Variables|Default|GetSteel%20frame%20movement))
  (bind _open_door (Variables|Default|Getopen%20door))
  (bind _returnvalue (Transformation|GetActorLocation _steel_frame_movement))
  (bind _returnvalue_2 (Transformation|GetActorLocation _open_door))
  (Utilities|FlowControl|Sequence
    (:then_0
      (Utilities|Casting|CastToBP_Projectile_Water OtherActor)
      (bind _move_value (Timeline|时间轴_0 Play)
        (:Update
          (Transformation|SetActorLocation _steel_frame_movement (Math|Vector|MakeVector (.x _returnvalue) (.y _returnvalue) (Math|Float|Lerp (.z _returnvalue) 1209.0 _move_value)) false false)
          (Utilities|FlowControl|Delay 3.0)
          (bind _blend_value (Timeline|时间轴 Play)
            (:Update
              (bind _returnvalue_3 (Rendering|Material|CreateDynamicMaterialInstance (Actor|GetComponentbyClass (Variables|Default|Getchange%20material) "/Script/Engine.StaticMeshComponent") 0 "/Game/Tan/Material/P2Door.P2Door" "Blend" :!class /Script/Engine.PrimitiveComponent))
              (Rendering|Material|SetScalarParameterValue _returnvalue_3 "Blend" _blend_value :!class /Script/Engine.MaterialInstanceDynamic)
              (Utilities|FlowControl|Delay 4.0)
              (bind _move_value_2 (Timeline|时间轴_2 Play)
                (:Update
                  (Transformation|SetActorLocation _open_door (Math|Vector|MakeVector (Math|Float|Lerp (.x _returnvalue_2) 5053.0 _move_value_2) (.y _returnvalue_2) (.z _returnvalue_2)) false false))
                (:Finished
                  (Utilities|FlowControl|Delay 0.2)
                  (Actor|DestroyActor (Variables|Default|Getopen%20door)))))))))
    (:then_1
      (Utilities|Casting|CastToBP_Cube_Player OtherActor)
      (Timeline|时间轴_0 Play))))

(event EventBeginPlay)

(event Collision|EventActorBeginOverlap
  (params (OtherActor :type Actor%20Object%20Reference)))

(event EventTick
  (params (DeltaSeconds :type Float%20%28single-precision%29)))

(fn ConstructionScript)