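; BP_WashingLiquid is a collectable that restores one point of Health to the cube player.
; Its Box overlap checks for the Player tag, casts to BP_Cube_Player and increments Health only when it differs from HealthMax.
; After healing, it destroys itself only if CanConsume is set; otherwise it stays in the level.
; Each branch outcome prints a debug string.
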(event OnComponentBeginOverlap(Box)
  (params (OverlappedComponent :type Primitive%20Component%20Object%20Reference) (OtherActor :type Actor%20Object%20Reference) (OtherComp :type Primitive%20Component%20Object%20Reference) (OtherBodyIndex :type Integer) (bFromSweep :type Boolean) (SweepResult :type Hit%20Result%20Structure%20%28by%20ref%29))
  (if (Actor|ActorHasTag OtherActor "Player")
    (bind _asbp_cube_player (Utilities|Casting|CastToBP_Cube_Player OtherActor)
      (:then
        (if (!= (Variables|/Game/Weihan/BP/Character/BP_Cube_Player.BP_Cube_Player_C|GetHealth _asbp_cube_player) (Variables|/Game/Weihan/BP/Character/BP_Cube_Player.BP_Cube_Player_C|GetHealth_Max _asbp_cube_player))
          (Math|Integer|IncrementInt (Variables|/Game/Weihan/BP/Character/BP_Cube_Player.BP_Cube_Player_C|GetHealth _asbp_cube_player)
            (:%20%20
              (if (Variables|Default|GetCanConsume?)
                (Development|PrintString "Hello")
                (Actor|DestroyActor)
                (else
                  (Development|PrintString "4444")))))
          (else
            (Development|PrintString "3333"))))
      (:CastFailed
        (Development|PrintString "2222")))
    (else
      (Development|PrintString "1111"))))

(event EventBeginPlay
  (|CallParentFunction) ; 此节点被禁用，将不会被调用。\n从引脚连出引线来编译功能。
)

(event Collision|EventActorBeginOverlap
  (params (OtherActor :type Actor%20Object%20Reference))
  (|CallParentFunction OtherActor) ; 此节点被禁用，将不会被调用。\n从引脚连出引线来编译功能。
)

(event EventTick
  (params (DeltaSeconds :type Float%20%28single-precision%29))
  (|CallParentFunction DeltaSeconds) ; 此节点被禁用，将不会被调用。\n从引脚连出引线来编译功能。
)

(fn ConstructionScript
  (|CallParentFunction))