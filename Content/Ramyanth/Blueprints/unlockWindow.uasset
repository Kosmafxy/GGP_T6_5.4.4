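; Blueprint actor that unlocks a window after being shot with water projectiles.
; Its Box overlap event counts overlaps from BP_Projectile_Water actors.
; On the fourth hit it latches HasTriggered and shifts a referenced TargetActor by a fixed local rotation and offset, with no animation, so it fires only once.
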(event OnComponentBeginOverlap(Box)
  (params (OverlappedComponent :type Primitive%20Component%20Object%20Reference) (OtherActor :type Actor%20Object%20Reference) (OtherComp :type Primitive%20Component%20Object%20Reference) (OtherBodyIndex :type Integer) (bFromSweep :type Boolean) (SweepResult :type Hit%20Result%20Structure%20%28by%20ref%29))
  (Utilities|Casting|CastToBP_Projectile_Water OtherActor)
  (Utilities|Casting|CastToBP_Projectile_Water OtherActor)
  (if (not (Variables|Default|GetbHasTriggered))
    (bind _output_get (Variables|Default|SetHitCount (+ (Variables|Default|GetHitCount) 1)))
    (if (== _output_get 4)
      (Variables|Default|SetbHasTriggered true)
      (Transformation|AddActorLocalRotation (Variables|Default|GetTargetActor) "-25.000000,0.000000,0.000000" false false)
      (Transformation|AddActorLocalOffset (Variables|Default|GetTargetActor) "-315.000000,0.000000,0.000000" false false))))

(event EventBeginPlay)

(event Collision|EventActorBeginOverlap
  (params (OtherActor :type Actor%20Object%20Reference)))

(event EventTick
  (params (DeltaSeconds :type Float%20%28single-precision%29)))

(fn ConstructionScript)